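; Game mode for a brick-breaker game that runs the match state machine from ready and countdown through playing, pause, game over and completion.
; It counts bricks at start, and decrementing that count to zero completes the level and opens the next numbered level via the game instance.
; A lost ball checks paddle lives to choose retry or game over.
; Game over and game completion show a play-again widget.
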(event Custom|SetGameState
  (params (StateGame :type StateGameEnum%20Enum :default "NewEnumerator0"))
  (switch Utilities|FlowControl|Switch|SwitchonStateGameEnum StateGame
    (:NewEnumerator0
      (Variables|Default|SetStateofTheGame "NewEnumerator0"))
    (:NewEnumerator1
      (Variables|Default|SetCountDown 3.0)
      (Variables|Default|SetStateofTheGame "NewEnumerator1"))
    (:NewEnumerator2
      (Variables|Default|SetStateofTheGame "NewEnumerator2")
      (Utilities|FlowControl|Delay 1.0)
      (bind _asbp_paddle_pawn (Utilities|Casting|CastToBP_Paddle_Pawn (Game|Player|GetPlayerPawn 0)))
      (if (<= (Variables|/Game/Blueprints/BP_Paddle_Pawn.BP_Paddle_Pawn_C|GetBallLives _asbp_paddle_pawn) 0)
        (CallFunction|SetGameState "NewEnumerator3")
        (else
          (CallFunction|SetGameState "NewEnumerator0"))))
    (:NewEnumerator3
      (Variables|Default|SetStateofTheGame "NewEnumerator3")
      (Utilities|FlowControl|Delay 1.0)
      (CallFunction|AskPlayAgain))
    (:NewEnumerator4
      (Variables|Default|SetStateofTheGame "NewEnumerator4")
      (Utilities|FlowControl|Delay 1.0)
      (bind _asbp_game_instance (Utilities|Casting|CastToBP_GameInstance (Game|GetGameInstance)))
      (if (== (Variables|/Game/Blueprints/BP_GameInstance.BP_GameInstance_C|GetmaxLevels _asbp_game_instance) (Variables|/Game/Blueprints/BP_GameInstance.BP_GameInstance_C|GetcurrentLevel _asbp_game_instance))
        (CallFunction|SetGameState "NewEnumerator7")
        (else
          (bind _result (Math|Integer|IncrementInt (Variables|/Game/Blueprints/BP_GameInstance.BP_GameInstance_C|GetcurrentLevel _asbp_game_instance))
            (:%20%20
              (Game|OpenLevel(byName) (Utilities|String|StringToName (Utilities|String|Append "Level_" (Utilities|String|ToString(Integer) _result)))))))))
    (:NewEnumerator5
      (Default|CallStartPlaing)
      (Variables|Default|SetStateofTheGame "NewEnumerator5"))
    (:NewEnumerator6
      (Variables|Default|SetStateofTheGame "NewEnumerator6")
      (Game|SetGamePaused true))
    (:NewEnumerator7
      (Variables|Default|SetStateofTheGame "NewEnumerator7")
      (Utilities|FlowControl|Delay 1.0)
      (CallFunction|AskPlayAgain))))

(event EventBeginPlay
  (Variables|Default|SetStateofTheGame "NewEnumerator0")
  (bind _outactors (Actor|GetAllActorsOfClass "/Game/Blueprints/BP_Brick.BP_Brick_C"))
  (for _array_element _outactors
    (Math|Integer|IncrementInt (Variables|Default|GetcountBrick))))

(event EventTick
  (params (DeltaSeconds :type Float%20%28single-precision%29))
  (if (Utilities|Enum|Equal(Enum) (Variables|Default|GetStateofTheGame) "NewEnumerator1")
    (bind _output_get (Variables|Default|SetCountDown (- (Variables|Default|GetCountDown) DeltaSeconds)))
    (if (>= _output_get 2.0)
      (Variables|Default|Setcount 3)
      (elif (>= _output_get 1.0)
        (Variables|Default|Setcount 2)
        (elif (>= _output_get 0.0)
          (Variables|Default|Setcount 1)
          (else
            (CallFunction|SetGameState "NewEnumerator5")))))))

(fn ConstructionScript)

(fn AskPlayAgain
  (bind _returnvalue (Game|GetPlayerController 0))
  (bind _returnvalue_2 (UserInterface|CreateWidget "/Game/Widgets/BP_PlayAgain.BP_PlayAgain_C"))
  (bind _output_get (Variables|Default|SetPlayAgainWidget _returnvalue_2))
  (UserInterface|Viewport|AddtoViewport _output_get 0)
  (Variables|/Script/Engine.PlayerController|SetbShowMouseCursor _returnvalue true)
  (Input|SetInputModeUIOnly _returnvalue 0 "DoNotLock"))

(fn DecrementBrickCount
  (bind _result (Math|Integer|DecrementInt (Variables|Default|GetcountBrick))
    (:%20%20
      (if (<= _result 0)
        (CallFunction|SetGameState "NewEnumerator4")))))