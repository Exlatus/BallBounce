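; Player controller for a ball game that turns input actions into game state changes on BP_Ball_GameMode.
; LMBDown advances the game mode from its first enum state to the next, only while in that first state.
; Quit records PreviousState, then either enters a quit-prompt state and calls AskPlayAgain, or leaves that state for a fixed one.
; PreviousState is not read back in this Blueprint.
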(event EventBeginPlay)

(event EventTick
  (params (DeltaSeconds :type Float%20%28single-precision%29)))

(event Input|ActionEvents|InputActionLMBDown
  (params (Key :type Key%20Structure :default "None"))
  (:Pressed
    (bind _asbp_ball_game_mode (Utilities|Casting|CastToBP_Ball_GameMode (Game|GetGameMode)))
    (if (Utilities|Enum|Equal(Enum) (Variables|/Game/Blueprints/BP_Ball_GameMode.BP_Ball_GameMode_C|GetStateofTheGame _asbp_ball_game_mode) "NewEnumerator0")
      (Default|SetGameState _asbp_ball_game_mode "NewEnumerator1"))))

(event Input|ActionEvents|InputActionQuit
  (params (Key :type Key%20Structure :default "None"))
  (:Pressed
    (bind _asbp_ball_game_mode (Utilities|Casting|CastToBP_Ball_GameMode (Game|GetGameMode)))
    (Variables|Default|SetPrevious%20state (Variables|/Game/Blueprints/BP_Ball_GameMode.BP_Ball_GameMode_C|GetStateofTheGame _asbp_ball_game_mode))
    (if (Utilities|Enum|Equal(Enum) (Variables|/Game/Blueprints/BP_Ball_GameMode.BP_Ball_GameMode_C|GetStateofTheGame _asbp_ball_game_mode) "NewEnumerator6")
      (Default|SetGameState _asbp_ball_game_mode "NewEnumerator5")
      (else
        (Default|SetGameState _asbp_ball_game_mode "NewEnumerator6")
        (Default|AskPlayAgain _asbp_ball_game_mode)))))

(fn ConstructionScript)