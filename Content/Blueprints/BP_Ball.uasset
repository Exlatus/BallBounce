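; Ball actor for a paddle-and-ball game, reset to a fixed spot with a randomized direction when the game mode signals play start.
; While the game mode is in a specific state, Tick moves it by a swept planar offset, not scaled by delta time.
; Blocking hits reflect the direction: paddle hits add paddle axis input and an X bias, while other hit actors implementing BP_HitInterface receive HitByBallMessage.
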(event Custom|BallStartPlaing
  (CallFunction|ResetBallPosition))

(event EventBeginPlay
  (bind _asbp_ball_game_mode (Utilities|Casting|CastToBP_Ball_GameMode (Game|GetGameMode)))
  (EventDispatchers|BindEventtoStartPlaing _asbp_ball_game_mode (delegate Custom|BallStartPlaing)))

(event Collision|EventActorBeginOverlap
  (params (OtherActor :type Actor%20Object%20Reference)))

(event EventTick
  (params (DeltaSeconds :type Float%20%28single-precision%29))
  (bind _asbp_ball_game_mode (Utilities|Casting|CastToBP_Ball_GameMode (Game|GetGameMode)))
  (if (Utilities|Enum|Equal(Enum) (Variables|/Game/Blueprints/BP_Ball_GameMode.BP_Ball_GameMode_C|GetStateofTheGame _asbp_ball_game_mode) "NewEnumerator5")
    (bind _sweephitresult (Transformation|AddActorWorldOffset (Math|Vector|MakeVector (.X (Math|Vector|BreakVector (* (Variables|Default|GetVectorDirection) (Variables|Default|GetSpeed)))) (.Y (Math|Vector|BreakVector (* (Variables|Default|GetVectorDirection) (Variables|Default|GetSpeed)))) 0.0) true))
    (if (.bBlockingHit (Collision|BreakHitResult _sweephitresult))
      (bind _asbp_paddle_pawn (Utilities|Casting|CastToBP_Paddle_Pawn (.HitActor (Collision|BreakHitResult _sweephitresult)))
        (:then
          (Variables|Default|SetVectorDirection (Math|Vector|Normalize (Math|Vector|MakeVector (+ (.X (Math|Vector|BreakVector (Math|Vector|Normalize (Math|Vector|MakeVector (.X (Math|Vector|BreakVector (Math|Vector|GetReflectionVector (Variables|Default|GetVectorDirection) (.ImpactNormal (Collision|BreakHitResult _sweephitresult))))) (+ (.Y (Math|Vector|BreakVector (Math|Vector|GetReflectionVector (Variables|Default|GetVectorDirection) (.ImpactNormal (Collision|BreakHitResult _sweephitresult))))) (* (Variables|/Game/Blueprints/BP_Paddle_Pawn.BP_Paddle_Pawn_C|GetAxisValue _asbp_paddle_pawn) 5.0)) (.Z (Math|Vector|BreakVector (Math|Vector|GetReflectionVector (Variables|Default|GetVectorDirection) (.ImpactNormal (Collision|BreakHitResult _sweephitresult))))))))) (Variables|Default|GetminX)) (.Y (Math|Vector|BreakVector (Math|Vector|Normalize (Math|Vector|MakeVector (.X (Math|Vector|BreakVector (Math|Vector|GetReflectionVector (Variables|Default|GetVectorDirection) (.ImpactNormal (Collision|BreakHitResult _sweephitresult))))) (+ (.Y (Math|Vector|BreakVector (Math|Vector|GetReflectionVector (Variables|Default|GetVectorDirection) (.ImpactNormal (Collision|BreakHitResult _sweephitresult))))) (* (Variables|/Game/Blueprints/BP_Paddle_Pawn.BP_Paddle_Pawn_C|GetAxisValue _asbp_paddle_pawn) 5.0)) (.Z (Math|Vector|BreakVector (Math|Vector|GetReflectionVector (Variables|Default|GetVectorDirection) (.ImpactNormal (Collision|BreakHitResult _sweephitresult))))))))) (.Z (Math|Vector|BreakVector (Math|Vector|Normalize (Math|Vector|MakeVector (.X (Math|Vector|BreakVector (Math|Vector|GetReflectionVector (Variables|Default|GetVectorDirection) (.ImpactNormal (Collision|BreakHitResult _sweephitresult))))) (+ (.Y (Math|Vector|BreakVector (Math|Vector|GetReflectionVector (Variables|Default|GetVectorDirection) (.ImpactNormal (Collision|BreakHitResult _sweephitresult))))) (* (Variables|/Game/Blueprints/BP_Paddle_Pawn.BP_Paddle_Pawn_C|GetAxisValue _asbp_paddle_pawn) 5.0)) (.Z (Math|Vector|BreakVector (Math|Vector|GetReflectionVector (Variables|Default|GetVectorDirection) (.ImpactNormal (Collision|BreakHitResult _sweephitresult)))))))))))))
        (:CastFailed
          (Variables|Default|SetVectorDirection (Math|Vector|GetReflectionVector (Variables|Default|GetVectorDirection) (.ImpactNormal (Collision|BreakHitResult _sweephitresult))))
          (if (Utilities|DoesObjectImplementInterface (.HitActor (Collision|BreakHitResult _sweephitresult)) "/Game/Blueprints/BP_HitInterface.BP_HitInterface_C")
            (Class|BPHitInterface|HitbyBall(Message) (.HitActor (Collision|BreakHitResult _sweephitresult)))))))))

(fn ConstructionScript)

(fn ResetBallPosition
  (Transformation|SetActorLocation "270.000000, 0, 0" false false)
  (Variables|Default|SetVectorDirection (Math|Vector|MakeVector 1.0 (Math|Random|RandomFloatinRange -1.0 1.0) 1.0)))