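; BP_Brick is a breakable brick for a ball-and-brick game that takes damage each time the ball hits it.
; On BeginPlay it creates a BP_BrickHitpoints widget with a reference to itself and assigns it to the NumberHitPoints component.
; HitbyBall lowers HitPoints and plays an impact sound.
; The final hit decrements the game mode's brick count, increments PlayerScore in the game instance and destroys the brick.
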(event EventHitbyBall
  (CallFunction|DecrementHitpoints)
  (Audio|PlaySound2D "/Game/Meshes/retro_impact_hit_11_Cue.retro_impact_hit_11_Cue" 1.0 1.0 0.0 0 0))

(event EventBeginPlay
  (bind _returnvalue (UserInterface|CreateWidget "/Game/Widgets/BP_BrickHitpoints.BP_BrickHitpoints_C"))
  (Variables|/Game/Widgets/BP_BrickHitpoints.BP_BrickHitpoints_C|SetrefToBrick _returnvalue self)
  (UserInterface|SetWidget (Variables|Default|GetNumber_HitPoints) _returnvalue))

(fn ConstructionScript)

(fn DecrementHitpoints
  (if (<= (- (Variables|Default|GetHitPoints) 1) 0)
    (bind _asbp_ball_game_mode (Utilities|Casting|CastToBP_Ball_GameMode (Game|GetGameMode)))
    (Default|DecrementBrickCount _asbp_ball_game_mode)
    (bind _asbp_game_instance (Utilities|Casting|CastToBP_GameInstance (Game|GetGameInstance)))
    (Math|Integer|IncrementInt (Variables|/Game/Blueprints/BP_GameInstance.BP_GameInstance_C|GetPlayerScore _asbp_game_instance)
      (:%20%20
        (Actor|DestroyActor)))
    (else
      (Math|Integer|DecrementInt (Variables|Default|GetHitPoints)))))